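; BP_Key is a keycard pickup that counts toward a collect-to-win goal.
; Its Box overlap with BP_ThirdPersonCharacter enables or disables the key's input for player 0.
; Pressing E decrements CollectablesLeft on the game mode, adds a W_Collectable widget, destroys the key and plays a sound.
; The game-mode cast limits pickup to the server, as the ClientPickup and EtoPickUpKey replication events are empty stubs.
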(event `ClientPickup`
  ;[1 1 1] Replication organisation
)

(event `E to Pick Up Key`
  ;[1 1 1] Picks up keycard, detects how many have been collected
)

(event `Key|E`
  (params (Key :type "Key Structure"))
  ;[1 1 1] Picks up keycard, detects how many have been collected
  (:`Pressed`
    (bind _asbp_third_person_game_mode (cast `/Game/ThirdPerson/Blueprints/BP_ThirdPersonGameMode` (`GameplayStatics.GetGameMode`)))
    (bind _result (`/Engine/EditorBlueprintResources/StandardMacros.DecrementInt` (`/Game/ThirdPerson/Blueprints/BP_ThirdPersonGameMode.Collectables Left` _asbp_third_person_game_mode))
      (:`  `
        (set `/Game/ThirdPerson/Blueprints/BP_ThirdPersonGameMode.Collectables Left` _result _asbp_third_person_game_mode)
        (bind _returnvalue (`|CreateWidget` "/Game/CollectToWin/W_Collectable.W_Collectable_C"))
        (`UserWidget.AddToViewport` _returnvalue 0)
        (`self.K2_DestroyActor`)
        (`GameplayStatics.PlaySoundAtLocation` "/Engine/VREditor/Sounds/UI/Flashlight_Switch.Flashlight_Switch" (0.0 0.0 0.0) (struct) 1.0 1.0 0.0 null null null null)))))

(event `self.Box.OnComponentBeginOverlap`
  (params (OverlappedComponent :type "PrimitiveComponent Object Reference") (OtherActor :type "Actor Object Reference") (OtherComp :type "PrimitiveComponent Object Reference") (OtherBodyIndex :type Integer) (bFromSweep :type Boolean) (SweepResult :type "HitResult Structure (by ref)"))
  ;[1 1 1] Detects player overlap
  (`KismetSystemLibrary.PrintString` "Only Server Can Pick Up")
  (cast `/Game/ThirdPerson/Blueprints/BP_ThirdPersonCharacter` OtherActor)
  (`self.EnableInput` (`GameplayStatics.GetPlayerController` 0)))

(event `self.Box.OnComponentEndOverlap`
  (params (OverlappedComponent :type "PrimitiveComponent Object Reference") (OtherActor :type "Actor Object Reference") (OtherComp :type "PrimitiveComponent Object Reference") (OtherBodyIndex :type Integer))
  ;[1 1 1] Detects player overlap
  (cast `/Game/ThirdPerson/Blueprints/BP_ThirdPersonCharacter` OtherActor)
  (`self.DisableInput` (`GameplayStatics.GetPlayerController` 0)))

(fn `UserConstructionScript`)