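; BP_Turret is an automated turret that tracks and fires laser projectiles at a Player-tagged actor inside its detection sphere.
; Entering starts looping timers that yaw the turret top toward the target and spawn BP_LaserProjectile with sound; leaving clears them.
; A timed line trace checks for the player but ends at a cast with no effect.
; Damage and Niagara effect nodes are disconnected.
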(event `TurretProjectile`
  ;[1 1 1] Shoot the projectile
  (`GameplayStatics.PlaySoundAtLocation` "/Game/MilitaryWeapDark/Sound/Rifle/Wavs/RifleB_Fire04.RifleB_Fire04" (`self.K2_GetActorLocation`) (struct) 1.0 1.0 0.0 null null null null)
  (`|SpawnActorFromClass` "/Game/Blueprints/PlayerBlueprints/BP_LaserProjectile.BP_LaserProjectile_C" (`SceneComponent.K2_GetComponentToWorld` (`self.SpawnPosition`)) "AlwaysSpawn" "MultiplyWithRoot" null null))

(event `self.Sphere.OnComponentBeginOverlap`
  (params (OverlappedComponent :type "PrimitiveComponent Object Reference") (OtherActor :type "Actor Object Reference") (OtherComp :type "PrimitiveComponent Object Reference") (OtherBodyIndex :type Integer) (bFromSweep :type Boolean) (SweepResult :type "HitResult Structure (by ref)"))
  (bind _returnvalue (`self.ActorHasTag` OtherActor "Player"))
  ;[1 1 1] When see player, set target
  (`self.SetActorTickEnabled` OtherActor true)
  (`/Engine/EditorBlueprintResources/StandardMacros.IsValid` OtherActor
    (:`Is Valid`
      (if _returnvalue
        (set `self.Target` OtherActor)
        (`self.Track Target`)
        (if _returnvalue
          (`self.TurretProjectile`)
          (bind _returnvalue_2 (`KismetSystemLibrary.K2_SetTimerDelegate` (delegate `TurretProjectile`) 1.0 true))
          (set `self.Timer` _returnvalue_2))))))

(event `self.Sphere.OnComponentEndOverlap`
  (params (OverlappedComponent :type "PrimitiveComponent Object Reference") (OtherActor :type "Actor Object Reference") (OtherComp :type "PrimitiveComponent Object Reference") (OtherBodyIndex :type Integer))
  ;[1 1 1] When player leaves, stop tracking target
  (`/Engine/EditorBlueprintResources/StandardMacros.IsValid` OtherActor
    (:`Is Valid`
      (if (`self.ActorHasTag` OtherActor "Player")
        (`self.Target`
          (:`then`
            (`KismetSystemLibrary.K2_ClearAndInvalidateTimerHandle` (`self.TimeRef`))
            (`KismetSystemLibrary.K2_ClearAndInvalidateTimerHandle` (`self.FireTime`))
            (`KismetSystemLibrary.K2_ClearAndInvalidateTimerHandle` (`self.Timer`)))
          (:`else`))))))

(event `Track Target`
  ;[1 1 1] Rotate Turret
  (bind _returnvalue (`KismetSystemLibrary.K2_SetTimerDelegate` (delegate `MoveTurret`) 0.05 true true))
  (set `self.TimeRef` _returnvalue)
  (`KismetSystemLibrary.PrintString` "Turretpart")
  (bind _returnvalue_2 (`KismetSystemLibrary.K2_SetTimerDelegate` (delegate `Shoot Turret`) 0.3 true true))
  (set `self.FireTime` _returnvalue_2))

(event `MoveTurret`
  (bind _target (`self.Target`))
  (bind (_returnvalue_roll _returnvalue_pitch _returnvalue_yaw) (`KismetMathLibrary.BreakRotator` (`KismetMathLibrary.RInterpTo` (`SceneComponent.RelativeRotation` (`self.TurretTop`)) (`KismetMathLibrary.FindLookAtRotation` (`self.K2_GetActorLocation`) (`self.K2_GetActorLocation` _target)) (`GameplayStatics.GetWorldDeltaSeconds`) 100.0)))
  ;[1 1 1] Rotate Turret
  (`/Engine/EditorBlueprintResources/StandardMacros.IsValid` _target
    (:`Is Valid`
      (`SceneComponent.K2_SetRelativeRotation` (`self.TurretTop`) (`KismetMathLibrary.MakeRotator` 0.0 0.0 _returnvalue_yaw) false false))))

(event `Shoot Turret`
  ;[1 1 1] Fire line trace
  (bind (_outhit _returnvalue) (`KismetSystemLibrary.LineTraceSingle` (+ (`self.K2_GetActorLocation`) (0.0 0.0 80.0)) (`self.K2_GetActorLocation` (`self.Target`)) "TraceTypeQuery2" true))
  (if _returnvalue
    (bind (_bblockinghit _binitialoverlap _time _distance _location _impactpoint _normal _impactnormal _physmat _hitactor) (`GameplayStatics.BreakHitResult` _outhit))
    (if (`self.ActorHasTag` _hitactor "Player")
      (cast `/Game/ThirdPerson/Blueprints/BP_ThirdPersonCharacter` _hitactor))))

(fn `UserConstructionScript`)