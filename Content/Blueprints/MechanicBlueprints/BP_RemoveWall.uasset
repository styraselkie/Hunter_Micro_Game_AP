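; BP_RemoveWall is a trigger actor that opens a linked door when something overlaps its Box component.
; The overlap calls OpenDoorWithButton on the DoorSelect reference without checking which actor entered.
; BeginPlay creates a W_ButtonPress prompt widget, marked as not working; the player-checked logic to show and remove it is disconnected and never runs.
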(event `self.ReceiveBeginPlay`
  ;[1 1 1] Not-working-widget
  (bind _returnvalue (`|CreateWidget` "/Game/UI_and_HUD/W_ButtonPress.W_ButtonPress_C"))
  (set `self.InteractWidget` _returnvalue))

(event `self.Box.OnComponentBeginOverlap`
  (params (OverlappedComponent :type "PrimitiveComponent Object Reference") (OtherActor :type "Actor Object Reference") (OtherComp :type "PrimitiveComponent Object Reference") (OtherBodyIndex :type Integer) (bFromSweep :type Boolean) (SweepResult :type "HitResult Structure (by ref)"))
  ;[1 1 1] Overlap, trigger door animation
  (`/Game/Blueprints/MechanicBlueprints/BP_DoorMove.OpenDoorWithButton` (`self.DoorSelect`)))

(fn `UserConstructionScript`)