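; Turret actor that tracks and fires at a Player-tagged actor entering its sphere trigger.
; Overlap starts looping timers that interpolate the top's yaw toward the target and line-trace to it; leaving clears them.
; A trace hitting the player spawns muzzle flash, smoke trail and impact effects.
; Shots are visual only, as the ApplyDamage logic is disconnected.
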(event `self.Sphere.OnComponentBeginOverlap`
  (params (OverlappedComponent :type "PrimitiveComponent Object Reference") (OtherActor :type "Actor Object Reference") (OtherComp :type "PrimitiveComponent Object Reference") (OtherBodyIndex :type Integer) (bFromSweep :type Boolean) (SweepResult :type "HitResult Structure (by ref)"))
  ;[1 1 1] When see player, set target
  (`/Engine/EditorBlueprintResources/StandardMacros.IsValid` OtherActor
    (:`Is Valid`
      (if (`self.ActorHasTag` OtherActor "Player")
        (set `self.Target` OtherActor)
        (`self.Track Target`)))))

(event `self.Sphere.OnComponentEndOverlap`
  (params (OverlappedComponent :type "PrimitiveComponent Object Reference") (OtherActor :type "Actor Object Reference") (OtherComp :type "PrimitiveComponent Object Reference") (OtherBodyIndex :type Integer))
  ;[1 1 1] When player leaves, stop tracking target
  (`/Engine/EditorBlueprintResources/StandardMacros.IsValid` OtherActor
    (:`Is Valid`
      (if (`self.ActorHasTag` OtherActor "Player")
        (`self.Target`
          (:`then`
            (`KismetSystemLibrary.K2_ClearAndInvalidateTimerHandle` (`self.TimeRef`))
            (`KismetSystemLibrary.K2_ClearAndInvalidateTimerHandle` (`self.FireTime`)))
          (:`else`))))))

(event `Track Target`
  ;[1 1 1] Rotate Turret
  (bind _returnvalue (`KismetSystemLibrary.K2_SetTimerDelegate` (delegate `MoveTurret`) 0.05 true true))
  (set `self.TimeRef` _returnvalue)
  (`KismetSystemLibrary.PrintString` "Turretpart")
  (bind _returnvalue_2 (`KismetSystemLibrary.K2_SetTimerDelegate` (delegate `Shoot Turret`) 0.3 true true))
  (set `self.FireTime` _returnvalue_2))

(event `MoveTurret`
  (bind _target (`self.Target`))
  (bind (_returnvalue_roll _returnvalue_pitch _returnvalue_yaw) (`KismetMathLibrary.BreakRotator` (`KismetMathLibrary.RInterpTo` (`SceneComponent.RelativeRotation` (`self.TurretTop`)) (`KismetMathLibrary.FindLookAtRotation` (`self.K2_GetActorLocation`) (`self.K2_GetActorLocation` _target)) (`GameplayStatics.GetWorldDeltaSeconds`) 100.0)))
  ;[1 1 1] Rotate Turret
  (`/Engine/EditorBlueprintResources/StandardMacros.IsValid` _target
    (:`Is Valid`
      (`SceneComponent.K2_SetRelativeRotation` (`self.TurretTop`) (`KismetMathLibrary.MakeRotator` 0.0 0.0 _returnvalue_yaw) false false))))

(event `Shoot Turret`
  ;[1 1 1] Fire line trace
  (bind (_outhit _returnvalue) (`KismetSystemLibrary.LineTraceSingle` (+ (`self.K2_GetActorLocation`) (0.0 0.0 80.0)) (`self.K2_GetActorLocation` (`self.Target`)) "TraceTypeQuery2" true))
  (if _returnvalue
    (bind (_bblockinghit _binitialoverlap _time _distance _location _impactpoint _normal _impactnormal _physmat _hitactor) (`GameplayStatics.BreakHitResult` _outhit))
    (if (`self.ActorHasTag` _hitactor "Player")
      ;[1 1 1] Particle FX
      (`GameplayStatics.SpawnEmitterAttached` "/Game/MilitaryWeapDark/FX/P_AssaultRifle_MuzzleFlash.P_AssaultRifle_MuzzleFlash" (`self.TurretTop`) "FireSocket" (0.0 0.0 0.0) (struct) (1.0 1.0 1.0) "SnapToTarget")
      (bind _returnvalue_2 (`GameplayStatics.SpawnEmitterAttached` "/Game/FX/SmokeBeam/P_SmokeTrail.P_SmokeTrail" (`self.TurretTop`) "FireSocket"))
      (`FXSystemComponent.SetVectorParameter` _returnvalue_2 "TargetTest" (`self.K2_GetActorLocation` (`self.Target`)))
      (`GameplayStatics.SpawnEmitterAtLocation` "/Game/MilitaryWeapDark/FX/P_Impact_Metal_Medium_01.P_Impact_Metal_Medium_01" _impactpoint))))

(fn `UserConstructionScript`)