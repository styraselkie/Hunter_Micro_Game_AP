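; BP_RemoveWall is an interactable button actor that opens the doors linked to it.
; A box overlap shows a button-press prompt widget, created at BeginPlay, while the player character is inside and removes it on exit.
; Its Interact event searches all BP_DoorMove actors and calls OpenDoor, passing the player, on each whose DoorValue equals its ButtonValue.
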(event `self.ReceiveBeginPlay`
  (bind _returnvalue (`|CreateWidget` "/Game/UI_and_HUD/W_ButtonPress.W_ButtonPress_C"))
  (set `self.InteractWidget` _returnvalue))

(event `self.Box.OnComponentBeginOverlap`
  (params (OverlappedComponent :type "PrimitiveComponent Object Reference") (OtherActor :type "Actor Object Reference") (OtherComp :type "PrimitiveComponent Object Reference") (OtherBodyIndex :type Integer) (bFromSweep :type Boolean) (SweepResult :type "HitResult Structure (by ref)"))
  (if (== OtherActor (`GameplayStatics.GetPlayerCharacter` 0))
    (`UserWidget.AddToViewport` (`self.InteractWidget`) 0)))

(event `self.Box.OnComponentEndOverlap`
  (params (OverlappedComponent :type "PrimitiveComponent Object Reference") (OtherActor :type "Actor Object Reference") (OtherComp :type "PrimitiveComponent Object Reference") (OtherBodyIndex :type Integer))
  (if (== OtherActor (`GameplayStatics.GetPlayerCharacter` 0))
    (`Widget.RemoveFromParent` (`self.InteractWidget`))))

(event `/Game/Blueprints/BP_InteractInterface.Interact`
  (params (Player :type "Character Object Reference"))
  (bind _outactors (`GameplayStatics.GetAllActorsOfClass` "/Game/Blueprints/BP_DoorMove.BP_DoorMove_C"))
  (for _array_element _outactors
    (if (== (`/Game/Blueprints/BP_DoorMove.DoorValue` _array_element) (`self.Button Value`))
      (`/Game/Blueprints/BP_DoorMove.OpenDoor` _array_element Player))))

(fn `UserConstructionScript`)