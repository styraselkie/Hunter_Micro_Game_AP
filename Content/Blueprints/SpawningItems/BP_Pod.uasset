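; BP_Pod is an interactable pod whose container switches between a glass and a glowy material when the player presses E nearby.
; A box trigger enables player input and toggles a text render on overlap begin, then disables input and toggles the text again on exit.
; A looping MultiGate on the E key alternates the material on one slot of the container.
; The overlap events do not check which actor triggered them.
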(event `self.Box.OnComponentBeginOverlap`
  (params (OverlappedComponent :type "PrimitiveComponent Object Reference") (OtherActor :type "Actor Object Reference") (OtherComp :type "PrimitiveComponent Object Reference") (OtherBodyIndex :type Integer) (bFromSweep :type Boolean) (SweepResult :type "HitResult Structure (by ref)"))
  (`self.EnableInput` (`GameplayStatics.GetPlayerController` 0))
  (`SceneComponent.ToggleVisibility` (`self.TextRender`) false :!label _label))

(event `self.Box.OnComponentEndOverlap`
  (params (OverlappedComponent :type "PrimitiveComponent Object Reference") (OtherActor :type "Actor Object Reference") (OtherComp :type "PrimitiveComponent Object Reference") (OtherBodyIndex :type Integer))
  (`self.DisableInput` (`GameplayStatics.GetPlayerController` 0))
  (goto _label))

(event `Key|E`
  (params (Key :type "Key Structure"))
  (bind _container (`self.Container`))
  (:`Pressed`
    (`|MultiGate` false true
      (:`Out 0`
        (`PrimitiveComponent.SetMaterial` _container 2 "/Game/Blueprints/OtherItems/Glass.Glass"))
      (:`Out 1`
        (`PrimitiveComponent.SetMaterial` _container 2 "/Game/Blueprints/M_GlowyObjects.M_GlowyObjects")))))

(fn `UserConstructionScript`)