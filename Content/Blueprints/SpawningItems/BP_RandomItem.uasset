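; BP_RandomItem is a placeable actor that spawns one random item when play begins.
; BeginPlay calls RandomObjects, which asks SpawningManager for a random class and spawns it using the DefaultSceneRoot's relative transform.
; An older approach that set a ChildActor class and a random yaw, along with a hardcoded item Select, remains in the graph but never runs.
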(event `self.ReceiveBeginPlay`
  ;[1 1 1] Spawn Random Actor
  (`self.RandomObjects`))

(event `RandomObjects`
  ;[1 1 1] Spawn Random Actor
  (`|SpawnActorFromClass` (`KismetArrayLibrary.Array_Random` (`self.SpawningManager`)) (`SceneComponent.GetRelativeTransform` (`self.DefaultSceneRoot`)) "Undefined" "MultiplyWithRoot" null null))

(fn `UserConstructionScript`)