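; PC_LocalMult is a player controller that, going by its name, serves local multiplayer and lets a player join the game.
; The IA_JoinGame Enhanced Input action prints a debug message, then has the game mode restart this player, whether or not a valid pawn is controlled.
; A delayed setup that would add the IMC_Default mapping context is left unconnected and never runs.
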(event `self.ReceiveBeginPlay`)

(event `EnhancedInput|/Game/ThirdPerson/Input/Actions/IA_JoinGame`
  (params (ActionValue :type Boolean) (ElapsedSeconds :type "Float (double-precision)") (TriggeredSeconds :type "Float (double-precision)") (InputAction :type "InputAction Object Reference" :default "/Game/ThirdPerson/Input/Actions/IA_JoinGame.IA_JoinGame"))
  (:`Triggered`
    (`KismetSystemLibrary.PrintString` "Joiend game")
    (`/Engine/EditorBlueprintResources/StandardMacros.IsValid` (`self.K2_GetPawn`)
      (:`Is Valid`
        _)
      (:`Is Not Valid`
        _))
    (`GameModeBase.RestartPlayer` (`GameplayStatics.GetGameMode`) self)))

(fn `UserConstructionScript`)